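; HUD for the boss raid mode that draws a crosshair and shows the player and boss HP/MP widgets.
; DrawHUD renders two black lines crossing at screen center, sized by AimLength.
; BeginPlay binds to the GameState's content-state change dispatcher and also runs the handler on the current state.
; When the state matches the target value (fade-in, per the comment), the handler creates both widgets and adds them to the viewport.
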(event `self.ReceiveDrawHUD`
  (params (SizeX :type Integer) (SizeY :type Integer))
  ;[1 1 1] 중간X값
  (set `self.CenterX` (/ SizeX 2))
  ;[1 1 1] 중간Y값
  (set `self.CenterY` (/ SizeY 2))
  ;[1 1 1] 에임 가로선
  (`self.DrawLine` (`KismetMathLibrary.Conv_IntToDouble` (- (`self.CenterX`) (`self.AimLength`))) (`KismetMathLibrary.Conv_IntToDouble` (`self.CenterY`)) (`KismetMathLibrary.Conv_IntToDouble` (+ (`self.CenterX`) (`self.AimLength`))) (`KismetMathLibrary.Conv_IntToDouble` (`self.CenterY`)) (struct :`A` 1.0) 5.0)
  ;[1 1 1] 에임 세로선
  (`self.DrawLine` (`KismetMathLibrary.Conv_IntToDouble` (`self.CenterX`)) (`KismetMathLibrary.Conv_IntToDouble` (+ (`self.CenterY`) (`self.AimLength`))) (`KismetMathLibrary.Conv_IntToDouble` (`self.CenterX`)) (`KismetMathLibrary.Conv_IntToDouble` (- (`self.CenterY`) (`self.AimLength`))) (struct :`A` 1.0) 5.0))

(event `self.ReceiveBeginPlay`
  ;[1 1 1] Call되었을 때, Content State가 Fadein이면 BossHp, PlayerHP Widget
  (bind _asbp_boss_raid_game_state (cast `/Game/BossRaidGame/GameMode/BP_BossRaid_GameState` (`GameplayStatics.GetGameState`)))
  (add `/Game/BossRaidGame/GameMode/BP_BossRaid_GameState.NewEventDispatcherChangeContentState` _asbp_boss_raid_game_state (`|CreateDelegate` :!event `BP Boss Raid HUD Auto Gen Func`))
  (`self.BP Boss Raid HUD Auto Gen Func` (`/Game/BossRaidGame/GameMode/BP_BossRaid_GameState.ContentState` _asbp_boss_raid_game_state)))

(fn `BP Boss Raid HUD Auto Gen Func`
  (params (NewParam :type "/Game/BossRaidGame/GameMode/EN_BossRaid_GameState Enum" :default "NewEnumerator0"))
  (if (`|EnumEquality` NewParam "NewEnumerator3")
    (bind _returnvalue (`|CreateWidget` "/Game/BossRaidGame/Widget/WG_PlayerHpMp.WG_PlayerHpMp_C"))
    (bind _output_get (set `self.PlayerHpMP` _returnvalue))
    (`UserWidget.AddToViewport` _output_get 0)
    (bind _returnvalue_2 (`|CreateWidget` "/Game/BossRaidGame/Widget/WG_BossHpMp.WG_BossHpMp_C"))
    (bind _output_get_2 (set `self.BossHPMP` _returnvalue_2))
    (`UserWidget.AddToViewport` _output_get_2 0)))

(fn `UserConstructionScript`)