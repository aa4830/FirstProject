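; Baby green dragon enemy that chases the player until its health runs out.
; BeginPlay fills health and re-issues AIMoveTo on a short delay loop, stopping movement once the death flag is set.
; Tick calls CallGreenDragonABP with a move flag and the player's 2D distance when within range.
; Overlapping bullets apply fixed damage, which AnyDamage subtracts from health to set the death flag.
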(event `self.ReceiveTick`
  (params (DeltaSeconds :type "Float (single-precision)"))
  (bind _asbp_boss_raid_character (cast `/Game/BossRaidGame/GameMode/BP_BossRaidCharacter` (`GameplayStatics.GetPlayerCharacter` 0)))
  (bind _returnvalue (`KismetMathLibrary.Vector_Distance2D` (`self.K2_GetActorLocation` _asbp_boss_raid_character) (`self.K2_GetActorLocation`)))
  (if (<= _returnvalue 2500.0)
    (`self.GreenDragon_ABP` true _returnvalue)))

(event `self.ReceiveBeginPlay`
  (set `self.CurrentHp` (`self.MaxHp`))
  (`|AIMoveTo` self (0.0 0.0 0.0) (`GameplayStatics.GetPlayerPawn` 0) :!label _label
    (:`then`
      _)
    (:`OnSuccess`
      _)
    (:`OnFail`
      _))
  (if (`self.IsDie`)
    (`MovementComponent.StopMovementImmediately` (`self.CharacterMovement`))
    (else
      (`KismetSystemLibrary.Delay` 0.2)
      (goto _label))))

(event `self.ReceiveAnyDamage`
  (params (Damage :type "Float (single-precision)") (DamageType :type "DamageType Object Reference") (InstigatedBy :type "Controller Object Reference") (DamageCauser :type "Actor Object Reference"))
  (set `self.CurrentHp` (`KismetMathLibrary.FClamp` (- (`self.CurrentHp`) Damage) 0.0 (`self.MaxHp`)))
  (if (<= (`self.CurrentHp`) 0.0)
    (set `self.IsDie` true)))

(event `self.ReceiveActorBeginOverlap`
  (params (OtherActor :type "Actor Object Reference"))
  (cast `/Game/BossRaidGame/Blueprints/BP_Bullet` OtherActor)
  (`GameplayStatics.ApplyDamage` self 10.0))

(fn `UserConstructionScript`)