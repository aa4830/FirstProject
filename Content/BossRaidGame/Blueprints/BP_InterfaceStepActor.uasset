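; BP_InterfaceStepActor is a step actor that brings up the start interface when its step begins.
; It extends the parent's start and end step events, creating WG_StartInterface on start, storing it as StartWidget and adding it to the viewport.
; Its separate Widget component is hidden on BeginPlay and again when the step ends, while StartWidget is not removed here.
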(event `self.ReceiveBeginPlay`
  (`parent.ReceiveBeginPlay`)
  (`SceneComponent.SetVisibility` (`self.Widget`) false false))

(fn `EventEndStep`
  (`parent.EventEndStep`)
  (`SceneComponent.SetVisibility` (`self.Widget`) false false))

(fn `EventStartStep`
  (`parent.EventStartStep`)
  (bind _returnvalue (`|CreateWidget` "/Game/BossRaidGame/Widget/WG_StartInterface.WG_StartInterface_C"))
  (bind _output_get (set `self.StartWidget` _returnvalue))
  (`UserWidget.AddToViewport` _output_get 0))

(fn `UserConstructionScript`
  (`parent.UserConstructionScript`))