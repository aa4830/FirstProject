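; BP_SelectBossStep is a step Blueprint that presents the boss selection screen when the step starts.
; On BeginPlay it hides its Widget component after running the parent logic.
; EventStartStep creates a WG_SelectBoss widget, stores it in SelectWidget and adds it to the viewport.
; EventEndStep only calls the parent and does not remove that widget itself.
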(event `self.ReceiveBeginPlay`
  (`parent.ReceiveBeginPlay`)
  (`SceneComponent.SetVisibility` (`self.Widget`) false false))

(fn `EventEndStep`
  (`parent.EventEndStep`))

(fn `EventStartStep`
  (`parent.EventStartStep`)
  (bind _returnvalue (`|CreateWidget` "/Game/BossRaidGame/Widget/WG_SelectBoss.WG_SelectBoss_C"))
  (bind _output_get (set `self.SelectWidget` _returnvalue))
  (`UserWidget.AddToViewport` _output_get 0))

(fn `UserConstructionScript`
  (`parent.UserConstructionScript`))