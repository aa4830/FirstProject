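; Boss red dragon Blueprint that turns to face the player every tick and runs a looping timer calling SpawnFireBall.
; Bullet overlaps apply fixed damage to itself, wake it and notify the boss animation Blueprint through a dispatcher.
; Damage handling scales up its particle system, clamps HP, flags death at zero and sends HP to the boss widget through another dispatcher.
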(event `self.ReceiveTick`
  (params (DeltaSeconds :type "Float (single-precision)"))
  ;[1 1 1] Tick마다 Player방향으로 회전함
  (`self.K2_SetActorRotation` (`KismetMathLibrary.FindLookAtRotation` (`self.K2_GetActorLocation` self) (`self.K2_GetActorLocation` (`GameplayStatics.GetPlayerPawn` 0)))))

(event `self.ReceiveActorBeginOverlap`
  (params (OtherActor :type "Actor Object Reference"))
  ;[1 1 1] Bullet에 Overlap되면, Apply Damage, Apply Widget Boss Widget, Set Is Wake Up
  (cast `/Game/BossRaidGame/Blueprints/BP_Bullet` OtherActor)
  (`GameplayStatics.ApplyDamage` self 10.0)
  (`self.Boss_ABP_Dispatcher` true)
  (set `self.IsWakeUp` true))

(event `self.ReceiveAnyDamage`
  (params (Damage :type "Float (single-precision)") (DamageType :type "DamageType Object Reference") (InstigatedBy :type "Controller Object Reference") (DamageCauser :type "Actor Object Reference"))
  (bind _returnvalue (`KismetMathLibrary.FClamp` (- (`self.CurrentHp`) Damage) 0.0 (`self.MaxHp`)))
  ;[1 1 1] Damage를 받으면 WG Boss Current Hp Apply, Hp <= 0 = Set Is Die
  (if (<= _returnvalue 80.0)
    _
    (else
      _))
  (`SceneComponent.SetWorldScale3D` (`self.ParticleSystem`) (* (`SceneComponent.RelativeScale3D` (`self.ParticleSystem`)) 15.0))
  (if (<= _returnvalue 0.0)
    (set `self.IsDie` true))
  (bind _output_get (set `self.CurrentHp` _returnvalue))
  (`self.Boss_WG_Dispatcher` _output_get (`self.MaxHp`)))

(event `self.ReceiveBeginPlay`
  ;[1 1 1] 시작하면, SpawnFireBall
  (set `self.CurrentHp` (`self.MaxHp`))
  (`KismetSystemLibrary.K2_SetTimer` null "SpawnFireBall" 6.0 true))

(fn `UserConstructionScript`
  (`parent.UserConstructionScript`))