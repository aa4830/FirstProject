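; Green dragon boss for the boss raid game, which fires projectiles and takes damage from player bullets.
; A looping timer spawns short-lived BP_FireBall actors from the FireFallForward component until the boss is dead.
; Overlapping a BP_Bullet applies fixed damage to itself, and AnyDamage clamps health, flags death at zero and broadcasts health through CallBossWGDispatcher.
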(event `self.ReceiveBeginPlay`
  (set `self.CurrentHp` (`self.MaxHp`))
  (`KismetSystemLibrary.K2_SetTimer` null "SpawnFireBall" 3.0 true))

(event `self.ReceiveAnyDamage`
  (params (Damage :type "Float (single-precision)") (DamageType :type "DamageType Object Reference") (InstigatedBy :type "Controller Object Reference") (DamageCauser :type "Actor Object Reference"))
  (bind _returnvalue (`KismetMathLibrary.FClamp` (- (`self.CurrentHp`) Damage) 0.0 (`self.MaxHp`)))
  (if (<= _returnvalue 0.0)
    (set `self.IsDie` true))
  (bind _output_get (set `self.CurrentHp` _returnvalue))
  (`self.Boss_WG_Dispatcher` _output_get (`self.MaxHp`)))

(event `self.ReceiveActorBeginOverlap`
  (params (OtherActor :type "Actor Object Reference"))
  (cast `/Game/BossRaidGame/Blueprints/BP_Bullet` OtherActor)
  (`GameplayStatics.ApplyDamage` self 10.0))

(fn `SpawnFireBall`
  (if (not (`self.IsDie`))
    (bind _returnvalue (`|SpawnActorFromClass` "/Game/BossRaidGame/Blueprints/BP_FireBall.BP_FireBall_C" (`SceneComponent.K2_GetComponentToWorld` (`self.FireFallForward`)) "Undefined" "MultiplyWithRoot" null self))
    (`self.SetLifeSpan` _returnvalue 3.0)))

(fn `UserConstructionScript`)