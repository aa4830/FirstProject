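; BP_StepActor is a step in the boss raid content flow, tied to the BP_BossRaid_GameState content state.
; On BeginPlay it binds to the game state's content-state change dispatcher and calls EventStartStep when the new state matches its CurrentStep.
; EventStartStep is empty here; EventEndStep advances the game state to NextStep, but its only call in this file is unwired.
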(event `self.ReceiveBeginPlay`
  (`self.BindGameState`))

(fn `BindGameState`
  (bind _asbp_boss_raid_game_state (cast `/Game/BossRaidGame/GameMode/BP_BossRaid_GameState` (`GameplayStatics.GetGameState`)))
  (add `/Game/BossRaidGame/GameMode/BP_BossRaid_GameState.NewEventDispatcherChangeContentState` _asbp_boss_raid_game_state (`|CreateDelegate` :!event `EventChangerContentState`)))

(fn `EventChangerContentState`
  (params (NewParam :type "/Game/BossRaidGame/GameMode/EN_BossRaid_GameState Enum" :default "NewEnumerator0"))
  (if (`|EnumEquality` NewParam (`self.CurrentStep`))
    (`self.EventStartStep`)))

(fn `EventEndStep`
  (bind _asbp_boss_raid_game_state (cast `/Game/BossRaidGame/GameMode/BP_BossRaid_GameState` (`GameplayStatics.GetGameState`)))
  (`/Game/BossRaidGame/GameMode/BP_BossRaid_GameState.ChangeContentState` _asbp_boss_raid_game_state (`self.NextStep`)))

(fn `EventStartStep`)

(fn `UserConstructionScript`)